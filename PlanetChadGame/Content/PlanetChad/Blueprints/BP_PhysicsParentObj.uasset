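; BP_PhysicsParentObj is a physics object base that simulates mutual gravitational attraction and repulsion between masses in the level.
; It copies the active mass list from BP_Player at BeginPlay, refreshes it on UpdateMassList, and removes itself when destroyed.
; Each Tick it applies inverse-square forces from every other mass, scaled by both masses and the other's mass-squared MaxGrav.
; IsRepulsor flips the direction, and a minimum distance clamp limits close-range force.
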(event `self.ReceiveBeginPlay`
  (bind _returnvalue (`PrimitiveComponent.GetMass` (`self.StaticMesh`)))
  ;[1 1 1] Gets Current List of Masses in level
  (bind _returnvalue_2 (`GameplayStatics.GetActorOfClass` "/Game/PlanetChad/Blueprints/BP_Player.BP_Player_C"))
  (bind _output_get (set `self.Player` _returnvalue_2))
  (set `self.MassesInLevel` (`/Game/PlanetChad/Blueprints/BP_Player.ActiveMasses` _output_get))
  ;[1 1 1] Set Gravity Strength Based on Mass
  (set `self.maxGrav` (* (`KismetMathLibrary.MultiplyMultiply_FloatFloat` _returnvalue 2.0) 1.0))
  (set `self.GravityStr` (* _returnvalue (`self.GravityConstant`))))

(event `UpdateMassList`
  ;[1 1 1] Updates MassesInLevel (called from BP_Player)
  (set `self.MassesInLevel` (`/Game/PlanetChad/Blueprints/BP_Player.ActiveMasses` (`self.Player`))))

(event `self.ReceiveDestroyed`
  ;[1 1 1] Remove self from global list
  (`/Game/PlanetChad/Blueprints/BP_Player.RemoveMass` (`self.Player`) self))

(event `self.ReceiveTick`
  (params (DeltaSeconds :type "Float (single-precision)"))
  (bind _returnvalue (`SceneComponent.K2_GetComponentLocation` (`self.StaticMesh`)))
  ;[1 1 1] Adding Gravity Forces
  (for _array_element (`self.MassesInLevel`)
    (if (!= _array_element self)
      (if (not (`/Game/PlanetChad/Blueprints/BP_PhysicsParentObj.IsRepulsor` _array_element))
        (bind _returnvalue_2 (`SceneComponent.K2_GetComponentLocation` (`Actor.RootComponent` _array_element)))
        (bind _returnvalue_3 (/ (* (`PrimitiveComponent.GetMass` (`/Game/PlanetChad/Blueprints/BP_PhysicsParentObj.StaticMesh` _array_element)) (`PrimitiveComponent.GetMass` (`self.StaticMesh`)) (`/Game/PlanetChad/Blueprints/BP_PhysicsParentObj.maxGrav` _array_element)) (`KismetMathLibrary.Square` (`KismetMathLibrary.FMax` (`self.GetDistanceTo` _array_element) 1000.0))))
        (set `self.Force` (* (`KismetMathLibrary.Normal` (- _returnvalue_2 _returnvalue)) _returnvalue_3))
        (else
          (set `self.Force` (* (`KismetMathLibrary.Normal` (- _returnvalue _returnvalue_2)) _returnvalue_3))))
      (`PrimitiveComponent.AddForce` (`self.StaticMesh`) (`self.Force`) "None" false))))

(fn `UserConstructionScript`)