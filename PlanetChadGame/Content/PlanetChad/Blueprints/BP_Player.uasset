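; Player pawn for PlanetChad that flies on input axes under a height cap and places masses in the world with the mouse.
; Clicks trace from the cursor; on a floor or non-end zone, left spawns a BP_Sphere and right a BP_Chad, sized by the game mode's UI.
; It tracks active masses, telling each to refresh its list of the others whenever one is added or removed.
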(event `InputAxis|MoveUp`
  (params (AxisValue :type "Float (single-precision)"))
  ;[1 1 1] Movement
  ;;[1 1 1] Space move up, left-shift move down
  (`self.K2_AddActorWorldOffset` (`KismetMathLibrary.MakeVector` 0.0 0.0 (* AxisValue (`self.SpeedMod`)))))

(event `InputAxis|MoveForward` :overrideparent false
  (params (AxisValue :type "Float (single-precision)"))
  ;[1 1 1] Movement
  ;;[1 1 1] W/S move forward/backward
  (`self.K2_AddActorWorldOffset` (`KismetMathLibrary.MakeVector` (* AxisValue (`self.SpeedMod`)))))

(event `InputAxis|MoveRight` :overrideparent false
  (params (AxisValue :type "Float (single-precision)"))
  ;[1 1 1] Movement
  ;;[1 1 1] A/D move left/right
  (`self.K2_AddActorWorldOffset` (`KismetMathLibrary.MakeVector` 0.0 (* AxisValue (`self.SpeedMod`)))))

(event `self.ReceiveTick`
  (params (DeltaSeconds :type "Float (single-precision)"))
  (bind _maxplayerzpoz (`self.MaxPlayerZPoz`))
  (bind _defaultsceneroot (`self.DefaultSceneRoot`))
  (bind (_returnvalue_x _returnvalue_y _returnvalue_z) (`KismetMathLibrary.BreakVector` (`SceneComponent.K2_GetComponentLocation` _defaultsceneroot)))
  ;[1 1 1] Limit height (so line trace always works)
  (if (> _returnvalue_z _maxplayerzpoz)
    (`SceneComponent.K2_SetWorldLocation` _defaultsceneroot (`KismetMathLibrary.MakeVector` _returnvalue_x _returnvalue_y _maxplayerzpoz) false false)))

(event `Key|LeftMouseButton`
  (params (Key :type "Key Structure"))
  (bind (_worldlocation _worlddirection) (`PlayerController.DeprojectMousePositionToWorld` (`GameplayStatics.GetPlayerController` 0)))
  ;[1 1 1] On left mouse button click, line trace downward (100000.0 cm) to find world pos, then spawn actor at that world pos if allowed
  (:`Pressed`
    (set `self.KeyPressed` Key)
    (bind _outhit (`KismetSystemLibrary.LineTraceSingle` _worldlocation (+ _worldlocation (* _worlddirection 100000.0)) "TraceTypeQuery1" :!label _label))
    ;;[1 1 1] If clicking on floor or start zone, spawn ball
    (cast `/Game/PlanetChad/Blueprints/BP_Floor` (`.HitActor` (`GameplayStatics.BreakHitResult` _outhit))
      (:`then`
        (if (== (`self.KeyPressed`) "LeftMouseButton") :!label _label_2
          (`self.Spawn Actor` (`.Location` (`GameplayStatics.BreakHitResult` _outhit)))
          (else
            (`self.Spawn Actor` (`.Location` (`GameplayStatics.BreakHitResult` _outhit)) "NewEnumerator1"))))
      (:`CastFailed`
        (bind _asbp_zone (cast `/Game/PlanetChad/Blueprints/BP_Zone` (`.HitActor` (`GameplayStatics.BreakHitResult` _outhit))))
        (if (not (`/Game/PlanetChad/Blueprints/BP_Zone.IsEndZone` _asbp_zone))
          (goto _label_2))))))

(event `Key|RightMouseButton`
  (params (Key :type "Key Structure"))
  ;[1 1 1] On left mouse button click, line trace downward (100000.0 cm) to find world pos, then spawn actor at that world pos if allowed
  (:`Pressed`
    (set `self.KeyPressed` Key)
    (goto _label)))

(event `RemoveMass`
  (params (DeletedSphere :type "/Game/PlanetChad/Blueprints/BP_PhysicsParentObj Object Reference"))
  ;[1 1 1] Updates Mass Lists when one is added or removed
  (`KismetArrayLibrary.Array_RemoveItem` (`self.ActiveMasses`) DeletedSphere)
  (`self.UpdateMassLists`))

(event `MassAdded`
  (params (AddedSphere :type "/Game/PlanetChad/Blueprints/BP_PhysicsParentObj Object Reference"))
  ;[1 1 1] Updates Mass Lists when one is added or removed
  (`KismetArrayLibrary.Array_Add` (`self.ActiveMasses`) AddedSphere)
  (`self.UpdateMassLists`))

(fn `SetMsses`
  (bind _outactors (`GameplayStatics.GetAllActorsOfClass` "/Game/PlanetChad/Blueprints/BP_PhysicsParentObj.BP_PhysicsParentObj_C"))
  (set `self.ActiveMasses` _outactors))

(fn `Spawn Actor`
  (params (SpawnLocation :type "Vector Structure") (SpawnActorType :type "/Game/PlanetChad/Blueprints/SpawnTypes Enum" :default "NewEnumerator0"))
  ;[1 1 1] Spawns actor at location
  (bind _asgm_planet_chad (cast `/Game/PlanetChad/Blueprints/GM_PlanetChad` (`GameplayStatics.GetGameMode`)))
  (if (`|EnumEquality` SpawnActorType "NewEnumerator0")
    (bind _returnvalue (`Slider.GetValue` (`/Game/PlanetChad/Blueprints/WBP_UI.Sizechoose` (`/Game/PlanetChad/Blueprints/GM_PlanetChad.UI Ref` _asgm_planet_chad))))
    (bind _returnvalue_2 (+ SpawnLocation (`KismetMathLibrary.MakeVector` 0.0 0.0 (* _returnvalue 50.0))))
    (bind _returnvalue_3 (`KismetMathLibrary.Conv_DoubleToVector` _returnvalue))
    ;;[1 1 1] Spawn BP_Sphere
    (bind _returnvalue_4 (`|SpawnActorFromClass` "/Game/PlanetChad/Blueprints/BP_Sphere.BP_Sphere_C" (`KismetMathLibrary.MakeTransform` _returnvalue_2 (struct) _returnvalue_3) "Undefined" "OverrideRootScale" null null))
    (`self.MassAdded` _returnvalue_4)
    (else
      ;;[1 1 1] Change to spawn repulsor
      (bind _returnvalue_5 (`|SpawnActorFromClass` "/Game/PlanetChad/Blueprints/BP_Chad.BP_Chad_C" (`KismetMathLibrary.MakeTransform` _returnvalue_2 (struct) _returnvalue_3) "Undefined" "OverrideRootScale" null null))
      (`self.MassAdded` _returnvalue_5))))

(fn `UpdateMassLists`
  ;[1 1 1] Updates Each Mass's List of other Masses.
  (for _array_element (`self.ActiveMasses`)
    (`/Game/PlanetChad/Blueprints/BP_Sphere.UpdateMassList` _array_element)))

(fn `UserConstructionScript`)